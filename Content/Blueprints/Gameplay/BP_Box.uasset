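; BP_Box is a breakable brick that can drop a random bonus pickup when hit.
; On BeginPlay it fills a Collectables array with speed, size and reset bonus classes.
; The first hit on its Brick component sets an IsPendingKill flag against repeat triggers, then destroys the actor.
; Before destruction, a random boolean decides whether SpawnBonus spawns a random class from the array at the brick's transform.
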(event `self.ReceiveBeginPlay`
  (bind _collectables (`self.Collectables`))
  (`KismetArrayLibrary.Array_Add` _collectables (`self.FastSpeedBonus`))
  (`KismetArrayLibrary.Array_Add` _collectables (`self.SlowSpeedBonus`))
  (`KismetArrayLibrary.Array_Add` _collectables (`self.SmallSizeBonus`))
  (`KismetArrayLibrary.Array_Add` _collectables (`self.LargeSizeBonus`))
  (`KismetArrayLibrary.Array_Add` _collectables (`self.ResetBonus`)))

(event `self.Brick.OnComponentHit`
  (params (HitComponent :type "PrimitiveComponent Object Reference") (OtherActor :type "Actor Object Reference") (OtherComp :type "PrimitiveComponent Object Reference") (NormalImpulse :type "Vector Structure") (Hit :type "HitResult Structure (by ref)"))
  (if (not (`self.IsPendingKill`))
    (set `self.IsPendingKill` true)
    (if (`KismetMathLibrary.RandomBool`)
      (`self.SpawnBonus` (`self.GetTransform` self)))
    (`self.K2_DestroyActor`)))

(fn `SpawnBonus`
  (params (Position :type "Transform Structure"))
  (`|SpawnActorFromClass` (`KismetArrayLibrary.Array_Random` (`self.Collectables`)) Position "Undefined" "OverrideRootScale" null null))

(fn `UserConstructionScript`)