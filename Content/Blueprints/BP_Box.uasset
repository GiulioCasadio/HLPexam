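; BP_Box is a breakable brick for an Arkanoid-style game, driven by hit events on its Brick component.
; Each hit decrements the brick count in ArkanoidGameState and destroys the actor while bricks remain.
; When the count reaches zero, it prints a win message and calls Restart on BP_ArkanoidGameMode instead.
; A SpawnBonus function is declared but empty.
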(event `self.Brick.OnComponentHit`
  (params (HitComponent :type "PrimitiveComponent Object Reference") (OtherActor :type "Actor Object Reference") (OtherComp :type "PrimitiveComponent Object Reference") (NormalImpulse :type "Vector Structure") (Hit :type "HitResult Structure (by ref)"))
  (bind _asarkanoid_game_state (cast `ArkanoidGameState` (`GameplayStatics.GetGameState`)))
  (`ArkanoidGameState.DecreaseBricks` _asarkanoid_game_state)
  (bind _returnvalue (`ArkanoidGameState.GetBricks` _asarkanoid_game_state))
  (if (== _returnvalue 0)
    (`KismetSystemLibrary.PrintString` "You Win")
    (bind _asbp_arkanoid_game_mode (cast `/Game/Blueprints/BP_ArkanoidGameMode` (`GameplayStatics.GetGameMode`)))
    (`/Game/Blueprints/BP_ArkanoidGameMode.Restart` _asbp_arkanoid_game_mode)
    (else
      (`self.K2_DestroyActor`))))

(fn `SpawnBonus`)

(fn `UserConstructionScript`)