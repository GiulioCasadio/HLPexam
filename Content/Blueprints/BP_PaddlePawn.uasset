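; Paddle pawn for an Arkanoid game that spawns a ball and holds it attached to itself.
; On BeginPlay it passes itself to SpawnBall on BP_ArkanoidGameMode.
; Its own SpawnBall event creates a Bp_Ball owned by the pawn at the Spawner component, stores it in BallRef and snaps it to that component.
; The graph contains no movement or launch logic.
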(event `self.ReceiveBeginPlay`
  (bind _asbp_arkanoid_game_mode (cast `/Game/Blueprints/BP_ArkanoidGameMode` (`GameplayStatics.GetGameMode`)))
  (`/Game/Blueprints/BP_ArkanoidGameMode.SpawnBall` _asbp_arkanoid_game_mode self))

(event `SpawnBall`
  (bind _returnvalue (`|SpawnActorFromClass` "/Game/Blueprints/Bp_Ball.Bp_Ball_C" (`SceneComponent.K2_GetComponentToWorld` (`self.Spawner`)) "Undefined" "OverrideRootScale" self null))
  (bind _output_get (set `self.ballRef` _returnvalue))
  (`/Engine/EditorBlueprintResources/StandardMacros.IsValid` _output_get
    (:`Is Valid`
      (`SceneComponent.K2_AttachToComponent` (`Actor.RootComponent` _output_get) (`self.Spawner`) "None" "SnapToTarget" "KeepRelative" "KeepWorld" true))))

(fn `UserConstructionScript`)