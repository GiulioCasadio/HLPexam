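; BP_Cornice is a boundary trigger in an Arkanoid game that removes balls overlapping its collider.
; On overlap it disables collision, destroys the overlapping actor and casts that actor's owner to the paddle pawn.
; It then has the game mode spawn a ball for that paddle, restores query-only collision and decreases the game state's ball count.
; A failed paddle or game mode cast leaves the collider disabled.
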(event `self.Collider.OnComponentBeginOverlap`
  (params (OverlappedComponent :type "PrimitiveComponent Object Reference") (OtherActor :type "Actor Object Reference") (OtherComp :type "PrimitiveComponent Object Reference") (OtherBodyIndex :type Integer) (bFromSweep :type Boolean) (SweepResult :type "HitResult Structure (by ref)"))
  (`self.DestroyBall` OtherActor))

(event `DestroyBall`
  (params (BallToDestroy :type "Actor Object Reference"))
  (bind _collider (`self.Collider`))
  (`PrimitiveComponent.SetCollisionEnabled` _collider "NoCollision")
  (bind _output_get (set `self.Player` (`self.GetOwner` BallToDestroy)))
  (`self.K2_DestroyActor` BallToDestroy)
  (bind _asbp_paddle_pawn (cast `/Game/Blueprints/BP_PaddlePawn` _output_get))
  (bind _asbp_arkanoid_game_mode (cast `/Game/Blueprints/BP_ArkanoidGameMode` (`GameplayStatics.GetGameMode`)))
  (`/Game/Blueprints/BP_ArkanoidGameMode.SpawnBall` _asbp_arkanoid_game_mode _asbp_paddle_pawn)
  (`PrimitiveComponent.SetCollisionEnabled` _collider "QueryOnly")
  (bind _asarkanoid_game_state (cast `ArkanoidGameState` (`GameplayStatics.GetGameState`)))
  (`ArkanoidGameState.DecreaseBalls` _asarkanoid_game_state))

(fn `UserConstructionScript`)